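; A collectible key actor that the first-person player picks up while overlapping it.
; Overlap begin and end set an in-range flag, show or remove a collect prompt widget and toggle the point light.
; The CollectKey event, if in range, destroys the actor, adds a key widget, plays a sound, triggers subtitles and sets CollectedKey on the cached player character.
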(event `self.ReceiveBeginPlay`
  ;[1 1 1] Initialize Object
  (set `self.newKey` false)
  (`SceneComponent.ToggleVisibility` (`self.PointLight`) false)
  (bind _asfirst_person_character (cast `/Game/FirstPersonBP/Blueprints/FirstPersonCharacter` (`GameplayStatics.GetPlayerCharacter` 0)))
  (set `self.FPC` _asfirst_person_character))

(event `self.ReceiveActorBeginOverlap`
  (params (OtherActor :type "Actor Object Reference"))
  ;[1 1 1] Initialize Collision
  (set `self.newKey` true)
  (bind _returnvalue (`|CreateWidget` "/Game/Blueprints/FToCollect.FToCollect_C" null null))
  (`UserWidget.AddToViewport` _returnvalue 0)
  (`SceneComponent.ToggleVisibility` (`self.PointLight`) false))

(event `self.ReceiveActorEndOverlap`
  (params (OtherActor :type "Actor Object Reference"))
  ;[1 1 1] Undo Initialization on End Collision
  (set `self.newKey` false)
  (bind _foundwidgets (`WidgetBlueprintLibrary.GetAllWidgetsOfClass` "/Game/Blueprints/FToCollect.FToCollect_C"))
  (`Widget.RemoveFromParent` _foundwidgets)
  (`SceneComponent.ToggleVisibility` (`self.PointLight`) false))

(event `CollectKey`
  ;[1 1 1] Collecting Key
  (if (`self.newKey`)
    (`self.K2_DestroyActor`)
    (bind _returnvalue (`|CreateWidget` "/Game/Blueprints/keyWidget.keyWidget_C"))
    (`UserWidget.AddToViewport` _returnvalue 0)
    (`GameplayStatics.PlaySound2D` "/Game/StarterContent/Audio/Collect.Collect" 1.0 1.0 0.0 null null)
    (bind _foundwidgets (`WidgetBlueprintLibrary.GetAllWidgetsOfClass` "/Game/Blueprints/subtitles.subtitles_C"))
    (`/Game/Blueprints/subtitles.collectKeySubtitles` _foundwidgets)
    (set `/Game/FirstPersonBP/Blueprints/FirstPersonCharacter.collectedKey` true (`self.FPC`))))

(fn `UserConstructionScript`)