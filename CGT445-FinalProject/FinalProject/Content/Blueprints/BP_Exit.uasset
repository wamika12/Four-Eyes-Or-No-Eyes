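; BP_Exit is the level exit actor that decides whether the player has finished the game's tasks.
; It caches the FirstPersonCharacter on BeginPlay.
; Any actor overlap checks that character's bag, book, key and brushing flags, without filtering which actor overlapped.
; If all are set, it clears all widgets and shows the winning widget; otherwise it calls TryAgain on the top-level Subtitles widgets.
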(event `self.ReceiveBeginPlay`
  ;[1 1 1] initialize
  (bind _asfirst_person_character (cast `/Game/FirstPersonBP/Blueprints/FirstPersonCharacter` (`GameplayStatics.GetPlayerCharacter` 0)))
  (set `self.FPC` _asfirst_person_character))

(event `self.ReceiveActorBeginOverlap`
  (params (OtherActor :type "Actor Object Reference"))
  (bind _fpc (`self.FPC`))
  (if (and (`/Game/FirstPersonBP/Blueprints/FirstPersonCharacter.collectedBag` _fpc) (`/Game/FirstPersonBP/Blueprints/FirstPersonCharacter.collectedBook` _fpc) (`/Game/FirstPersonBP/Blueprints/FirstPersonCharacter.collectedKey` _fpc) (`/Game/FirstPersonBP/Blueprints/FirstPersonCharacter.doneBrushing` _fpc))
    (`WidgetLayoutLibrary.RemoveAllWidgets`)
    (bind _returnvalue (`|CreateWidget` "/Game/Blueprints/winningWidget.winningWidget_C"))
    (`UserWidget.AddToViewport` _returnvalue 0)
    (else
      (bind _foundwidgets (`WidgetBlueprintLibrary.GetAllWidgetsOfClass` "/Game/Blueprints/subtitles.subtitles_C"))
      (`/Game/Blueprints/subtitles.tryAgain` _foundwidgets))))

(fn `UserConstructionScript`)