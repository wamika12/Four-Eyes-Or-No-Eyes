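; HUD Blueprint that shows the game's menus and runs a countup timer that ends the game.
; BeginPlay opens the start menu widget, and a separate event adds an FToCollect prompt to the viewport.
; Tick uses a Delay as a throttle, so Time rises about every five seconds until it triggers GameOver at its limit.
; GameOver pauses the game, clears all widgets and shows the game over widget.
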(event `self.ReceiveBeginPlay`
  ;[1 1 1] Start Game Menu
  (bind _returnvalue (`|CreateWidget` "/Game/Blueprints/StartGameWidget.StartGameWidget_C"))
  (`UserWidget.AddToViewport` _returnvalue 0))

(event `GameOver`
  ;[1 1 1] Creating Game Over Widget
  (`GameplayStatics.SetGamePaused` true)
  (`WidgetLayoutLibrary.RemoveAllWidgets`)
  (bind _returnvalue (`|CreateWidget` "/Game/Blueprints/gameOverWidget.gameOverWidget_C"))
  (`UserWidget.AddToViewport` _returnvalue 0))

(event `self.ReceiveTick`
  (params (DeltaSeconds :type "Float (single-precision)"))
  (bind _time (`self.time`))
  ;[1 1 1] Timer
  (`KismetSystemLibrary.Delay` 5.0)
  (set `self.time` (+ _time 1))
  (`/Engine/EditorBlueprintResources/StandardMacros.CompareInt` _time 30
    (:`==`
      (`self.GameOver`))))

(event `displayFToCollect`
  ;[1 1 1] displayFToCollect
  (bind _returnvalue (`|CreateWidget` "/Game/Blueprints/FToCollect.FToCollect_C" null null))
  (`UserWidget.AddToViewport` _returnvalue 0))

(fn `UserConstructionScript`)