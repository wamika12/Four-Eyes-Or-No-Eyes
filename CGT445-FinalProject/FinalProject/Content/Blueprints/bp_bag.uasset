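; Collectible bag actor that the first-person player picks up when standing near it.
; Overlap sets a proximity flag, shows a collect prompt widget and toggles the light's visibility, with end overlap clearing the flag and prompt and toggling again.
; The CollectBag event, when near, destroys the actor, shows the bag widget, triggers subtitles and sets CollectedBag on the cached character.
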(event `self.ReceiveBeginPlay`
  ;[1 1 1] Initialize Object
  (set `self.nearBag` false)
  (`SceneComponent.ToggleVisibility` (`self.light`) false)
  (bind _asfirst_person_character (cast `/Game/FirstPersonBP/Blueprints/FirstPersonCharacter` (`GameplayStatics.GetPlayerCharacter` 0)))
  (set `self.FPC` _asfirst_person_character))

(event `self.ReceiveActorBeginOverlap`
  (params (OtherActor :type "Actor Object Reference"))
  ;[1 1 1] Initialize Collision
  (set `self.nearBag` true)
  (bind _returnvalue (`|CreateWidget` "/Game/Blueprints/FToCollect.FToCollect_C" null null))
  (`UserWidget.AddToViewport` _returnvalue 0)
  (`SceneComponent.ToggleVisibility` (`self.light`) false))

(event `self.ReceiveActorEndOverlap`
  (params (OtherActor :type "Actor Object Reference"))
  ;[1 1 1] Undo Initialization on End Collision
  (set `self.nearBag` false)
  (bind _foundwidgets (`WidgetBlueprintLibrary.GetAllWidgetsOfClass` "/Game/Blueprints/FToCollect.FToCollect_C"))
  (`Widget.RemoveFromParent` _foundwidgets)
  (`SceneComponent.ToggleVisibility` (`self.light`) false))

(event `CollectBag`
  ;[1 1 1] CollectingBook
  (if (`self.nearBag`)
    (`self.K2_DestroyActor`)
    (bind _returnvalue (`|CreateWidget` "/Game/Blueprints/bagWidget.bagWidget_C"))
    (`UserWidget.AddToViewport` _returnvalue 0)
    (bind _foundwidgets (`WidgetBlueprintLibrary.GetAllWidgetsOfClass` "/Game/Blueprints/subtitles.subtitles_C"))
    (`/Game/Blueprints/subtitles.collecBagSubtitles` _foundwidgets)
    (set `/Game/FirstPersonBP/Blueprints/FirstPersonCharacter.collectedBag` true (`self.FPC`))))

(fn `UserConstructionScript`)