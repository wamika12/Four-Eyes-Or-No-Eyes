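; Door Blueprint that swings MyDoor open or closed when myDoorOpen is called while something overlaps its BoxCollision.
; Begin and end overlap set NearDoor, which gates a FlipFlop that alternately plays and reverses DoorRotationTimeline.
; Timeline updates drive the door's relative pitch, print a debug "Hello" and clear NearDoor, so another toggle requires a fresh overlap.
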(event `self.BoxCollision.OnComponentBeginOverlap`
  (params (OverlappedComponent :type "PrimitiveComponent Object Reference") (OtherActor :type "Actor Object Reference") (OtherComp :type "PrimitiveComponent Object Reference") (OtherBodyIndex :type Integer) (bFromSweep :type Boolean) (SweepResult :type "HitResult Structure (by ref)"))
  (set `self.nearDoor` true))

(event `self.BoxCollision.OnComponentEndOverlap`
  (params (OverlappedComponent :type "PrimitiveComponent Object Reference") (OtherActor :type "Actor Object Reference") (OtherComp :type "PrimitiveComponent Object Reference") (OtherBodyIndex :type Integer))
  (set `self.nearDoor` false))

(event `myDoorOpen`
  (if (`self.nearDoor`)
    (`/Engine/EditorBlueprintResources/StandardMacros.FlipFlop`
      (:`A`
        (bind (_direction _doorrotationamount) (`Timeline|DoorRotationTimeline` :!label _label)
          (:`Update`
            (`SceneComponent.K2_SetRelativeRotation` (`self.myDoor`) (`KismetMathLibrary.MakeRotator` 0.0 _doorrotationamount) false false)
            (`KismetSystemLibrary.PrintString` "Hello")
            (set `self.nearDoor` false))))
      (:`B`
        (goto _label :!via `Reverse`)))))

(fn `UserConstructionScript`)