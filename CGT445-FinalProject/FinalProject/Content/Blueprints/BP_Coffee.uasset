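; BP_Coffee is a coffee cup pickup that the first-person player drinks.
; Overlap arms it, toggles its point light and shows the FToCollect prompt.
; When armed, moveCup stops the player, snaps StaticMesh to the character's SphereTrans, clears the prompt and animates Cupcoffee along a spline via timeline.
; TrashCup, started alongside, destroys the actor after a delay and sets movement mode to Walking.
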(event `self.ReceiveBeginPlay`
  ;[1 1 1] Initialize Object
  (set `self.newCup` false)
  (`SceneComponent.ToggleVisibility` (`self.PointLight`) false))

(event `self.ReceiveActorBeginOverlap`
  (params (OtherActor :type "Actor Object Reference"))
  ;[1 1 1] Initialize Collision
  (set `self.newCup` true)
  (bind _returnvalue (`|CreateWidget` "/Game/Blueprints/FToCollect.FToCollect_C" null null))
  (`UserWidget.AddToViewport` _returnvalue 0)
  (`SceneComponent.ToggleVisibility` (`self.PointLight`) false))

(event `self.ReceiveActorEndOverlap`
  (params (OtherActor :type "Actor Object Reference"))
  ;[1 1 1] Undo Initialization on End Collision
  (set `self.newCup` false)
  (`SceneComponent.ToggleVisibility` (`self.PointLight`) false)
  (if (not (`self.doneDrinking`))
    (bind _foundwidgets (`WidgetBlueprintLibrary.GetAllWidgetsOfClass` "/Game/Blueprints/FToCollect.FToCollect_C"))
    (`Widget.RemoveFromParent` _foundwidgets)))

(event `moveCup`
  (bind _returnvalue (`GameplayStatics.GetPlayerCharacter` 0))
  (bind _spline (`self.Spline`))
  ;[1 1 1] Bursh Animation
  (`SceneComponent.ToggleVisibility` (`self.PointLight`) false)
  (if (`self.newCup`)
    (`self.trashCup`)
    (bind _asfirst_person_character (cast `/Game/FirstPersonBP/Blueprints/FirstPersonCharacter` _returnvalue))
    (set `self.FPT` _asfirst_person_character)
    (`MovementComponent.StopMovementImmediately` (`Character.CharacterMovement` _returnvalue))
    (`SceneComponent.K2_SetWorldTransform` (`self.StaticMesh`) (`SceneComponent.K2_GetComponentToWorld` (`/Game/FirstPersonBP/Blueprints/FirstPersonCharacter.SphereTrans` (`self.FPT`))) false false)
    (bind _foundwidgets (`WidgetBlueprintLibrary.GetAllWidgetsOfClass` "/Game/Blueprints/FToCollect.FToCollect_C"))
    (`Widget.RemoveFromParent` _foundwidgets)
    (bind (_direction _animationalpha) (`Timeline|Timeline_0`)
      (:`Update`
        (bind _returnvalue_2 (* (`SplineComponent.GetSplineLength` _spline) _animationalpha))
        (`SceneComponent.K2_SetWorldTransform` (`self.cup-coffee`) (`KismetMathLibrary.MakeTransform` (`SplineComponent.GetLocationAtDistanceAlongSpline` _spline _returnvalue_2 "World") (`SplineComponent.GetRotationAtDistanceAlongSpline` _spline _returnvalue_2 "World") (`SceneComponent.K2_GetComponentScale` (`self.cup-coffee`))) false false)))))

(event `trashCup`
  ;[1 1 1] Finish Brushing
  (`KismetSystemLibrary.Delay` 4.0)
  (`self.K2_DestroyActor`)
  (`CharacterMovementComponent.SetMovementMode` (`Character.CharacterMovement` (`GameplayStatics.GetPlayerCharacter` 0)) "MOVE_Walking" 0))

(fn `UserConstructionScript`)